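; Base enemy Blueprint that patrols, chases and melee-attacks the player, with an HP bar widget and montage death.
; BehaviourUnit switches on BehaviourMode, alternating random-point and nearest-patrol-point roaming until PawnSensing spots BP_Player.
; Chasing leads to a DoOnce-gated attack montage, whose notify fires a sphere trace for randomized damage while a recursive delay loop turns it toward the target.
; AnyDamage updates HP and the bar, destroying the actor at zero.
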(event `self.ReceiveBeginPlay`
  ;[1 1 1] 0703_add
  (`self.BehaviourUnit`)
  (bind _returnvalue (`|CreateWidget` "/Game/BP/UI/UBP_HPBar.UBP_HPBar_C" null (`self.HP`)))
  (bind _output_get (set `self.HPBar` _returnvalue))
  (`UserWidget.AddToViewport` _output_get 0))

(event `self.ReceiveTick`
  (params (DeltaSeconds :type "Float (single-precision)"))
  ;[1 1 1] 0703_add
  (bind _hpbar (`self.HPBar`)
    (:`then`
      (`/Game/BP/UI/UBP_HPBar.UpdateUILocation` _hpbar (`SceneComponent.K2_GetComponentLocation` (`self.UIPos`))))
    (:`else`)))

(event `BehaviourUnit`
  (bind _attackplayer_ (`self.AttackPlayer?`))
  (bind _charactermovement (`self.CharacterMovement`))
  (if (not (`self.IsDead?`))
    (switch `/Game/BP/BehaviourMode` (`self.BehaviourMode`)
      (:`NewEnumerator0`
        (`|AIMoveTo` self (`NavigationSystemV1.K2_GetRandomReachablePointInRadius` (`self.K2_GetActorLocation`) (`self.RoamRadius`) null null) null
          (:`OnSuccess`
            (`self.UpdatePatrolPoint`)
            (`KismetSystemLibrary.Delay` (`KismetMathLibrary.RandomFloatInRange` (`self.MinWait`) (`self.MaxWait`)))
            (if _attackplayer_
              (`self.ChasePlayer`)
              (else
                (set `self.BehaviourMode` "NewEnumerator1")
                (`self.BehaviourUnit`))))))
      (:`NewEnumerator1`
        (`|AIMoveTo` self (0.0 0.0 0.0) (`self.PatrolPointRef`)
          (:`OnSuccess`
            (if _attackplayer_
              (`self.ChasePlayer`)
              (else
                (`KismetSystemLibrary.Delay` (`KismetMathLibrary.RandomFloatInRange` (`self.MinWait`) (`self.MaxWait`)))
                (set `self.BehaviourMode` "NewEnumerator0")
                (`self.BehaviourUnit`))))))
      (:`NewEnumerator2`
        (if (not (`self.IsDead?`)) :!label _label
          (`|AIMoveTo` self (0.0 0.0 0.0) (`self.AttackTarget`) (`self.AttackAcceptanceRadius`)
            (:`OnSuccess`
              (`/Engine/EditorBlueprintResources/StandardMacros.DoOnce` false :!label _label_2
                (:`Completed`
                  (set `self.Attackingplayer?` true)
                  (bind _notifyname (`|PlayMontage` (`self.Mesh`) (`self.AttackMontage`))
                    (:`then`
                      (`MovementComponent.StopMovementImmediately` _charactermovement)
                      (set `CharacterMovementComponent.MaxWalkSpeed` 0.0 _charactermovement)
                      (`self.TrackPlayer`))
                    (:`OnCompleted`
                      (`KismetSystemLibrary.Delay` (`KismetMathLibrary.RandomFloatInRange` 0.1 0.3))
                      (set `self.Attackingplayer?` false)
                      (if (not (`self.IsDead?`))
                        (`self.ReleaseAttack`)
                        (set `CharacterMovementComponent.MaxWalkSpeed` 450.0 (`self.CharacterMovement`))
                        (`self.BehaviourUnit`)))
                    (:`OnNotifyBegin`
                      (switch `name` _notifyname
                        (:`AttackTrace`
                          (`self.AttckTrace`))))))))))))))

(event `self.PawnSensing.OnSeePawn`
  (params (Pawn :type "Pawn Object Reference"))
  (if (not (`self.IsDead?`))
    (bind _asbp_player (cast `/Game/GKnight/BP_Player` Pawn))
    (set `self.AttackTarget` _asbp_player)
    (set `self.BehaviourMode` "NewEnumerator2")
    (`self.BehaviourUnit`)))

(event `ChasePlayer`
  (goto _label))

(event `ReleaseAttack`
  (goto _label_2 :!via `Reset`))

(event `TrackPlayer`
  (bind (_returnvalue_roll _returnvalue_pitch _returnvalue_yaw) (`KismetMathLibrary.BreakRotator` (`KismetMathLibrary.FindLookAtRotation` (`self.K2_GetActorLocation`) (`self.K2_GetActorLocation` (`self.AttackTarget`)))))
  (`self.AttackTarget`
    (:`then`
      (if (`self.Attackingplayer?`)
        (`self.K2_SetActorRotation` (`KismetMathLibrary.MakeRotator` 0.0 0.0 _returnvalue_yaw))
        (`KismetSystemLibrary.Delay` 0.01)
        (`self.TrackPlayer`)))
    (:`else`)))

(event `self.ReceiveAnyDamage`
  (params (Damage :type "Float (single-precision)") (DamageType :type "DamageType Object Reference") (InstigatedBy :type "Controller Object Reference") (DamageCauser :type "Actor Object Reference"))
  ;[1 1 1] Adding_0703
  (bind _output_get (set `self.HP` (- (`self.HP`) Damage)))
  (`/Game/BP/UI/UBP_HPBar.OnTakeDamage` (`self.HPBar`) Damage)
  (if (<= _output_get 0.0)
    (`KismetSystemLibrary.Delay` 2.0)
    (`Widget.RemoveFromParent` (`self.HPBar`))
    (`|PlayMontage` (`self.Mesh`) (`self.Montage Death`)
      (:`OnCompleted`
        (`self.K2_DestroyActor`)))))

(event `self.ReceiveHit`
  (params (MyComp :type "PrimitiveComponent Object Reference") (Other :type "Actor Object Reference") (OtherComp :type "PrimitiveComponent Object Reference") (bSelfMoved :type Boolean) (HitLocation :type "Vector Structure") (HitNormal :type "Vector Structure") (NormalImpulse :type "Vector Structure") (Hit :type "HitResult Structure (by ref)"))
  ;[1 1 1] Adding_0703
)

(fn `AttckTrace`
  (bind _returnvalue (`self.K2_GetActorLocation`))
  (bind _attackdmg (`self.AttackDMG`))
  (bind (_outhit _returnvalue_2) (`KismetSystemLibrary.SphereTraceSingle` :`Start` _returnvalue :`End` (+ _returnvalue (* (`self.GetActorForwardVector`) (`self.AttackRange`))) :`Radius` (`self.AttackRadius`) :`TraceChannel` "TraceTypeQuery1" :`DrawDebugType` "ForDuration"))
  (if _returnvalue_2
    (`GameplayStatics.ApplyDamage` (`.HitActor` (`GameplayStatics.BreakHitResult` _outhit)) (`KismetMathLibrary.Conv_IntToDouble` (`KismetMathLibrary.Round` (`KismetMathLibrary.RandomFloatInRange` (- _attackdmg 2.0) (+ _attackdmg 2.0)))))))

(fn `UpdatePatrolPoint`
  (bind _outactors (`GameplayStatics.GetAllActorsOfClass` "/Game/BP/EnemyPatrolPoint_BP.EnemyPatrolPoint_BP_C"))
  (for _array_element _outactors
    (if (< (`self.GetDistanceTo` _array_element self) (`self.GetDistanceTo` (`self.PatrolPointRef`) self))
      (set `self.PatrolPointRef` _array_element))))

(fn `UserConstructionScript`
  (bind _outactors (`GameplayStatics.GetAllActorsOfClass` "/Game/BP/EnemyPatrolPoint_BP.EnemyPatrolPoint_BP_C"))
  (set `self.PatrolPointRef` (`|GetArrayItem` _outactors))
  (for _array_element _outactors
    (if (< (`self.GetDistanceTo` _array_element self) (`self.GetDistanceTo` (`self.PatrolPointRef`) self))
      (set `self.PatrolPointRef` _array_element))))